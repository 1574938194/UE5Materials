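; BP_Demo1 is a demo actor for an Excel spreadsheet (XLDocument) API.
; It enables player input on BeginPlay and calls RunDemoBasicUsage, whose body is not in this graph, when Q is pressed.
; An unconnected chain sketches the API flow from creating an xlsx at a hard-coded path through writing a cell to saving.
; A call to RunDemo1OLD is also left unwired.
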(event Collision|EventActorBeginOverlap
  (params (OtherActor :type Actor%20Object%20Reference)))

(event EventTick
  (params (DeltaSeconds :type Float%20%28single-precision%29)))

(event EventBeginPlay
  (Input|EnableInput (Game|GetPlayerController 0)))

(event Input|KeyboardEvents|Q
  (params (Key :type Key%20Structure :default "None"))
  (:Pressed
    (Class|Demo1|RunDemoBasicUsage)))

(fn ConstructionScript)